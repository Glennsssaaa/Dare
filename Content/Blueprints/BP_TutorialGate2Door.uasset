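; Door for the second tutorial gate that swings two panels open when its OpenGate event is called from outside.
; OpenGate disables collision on both static meshes, then plays a timeline that rotates Cube and Cube1 toward their own target rotations.
; Each update lerps from the current world rotation rather than a cached start, so the motion compounds instead of following the timeline curve directly.
; The file has no closing logic.
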(event Custom|OpenGate
  (bind _cube1 (Variables|Default|GetCube1))
  (bind _cube (Variables|Default|GetCube))
  (Collision|SetCollisionEnabled (Variables|Default|GetStaticMesh) "NoCollision")
  (Collision|SetCollisionEnabled (Variables|Default|GetStaticMesh1) "NoCollision")
  (bind _newtrack_0 (Timeline|Timeline Play)
    (:Update
      (Transformation|SetWorldRotation _cube (Math|Rotator|Lerp(Rotator) (Transformation|GetWorldRotation _cube) (Variables|Default|GetTargetRotation) _newtrack_0) false false)
      (Transformation|SetWorldRotation _cube1 (Math|Rotator|Lerp(Rotator) (Transformation|GetWorldRotation _cube1) (Variables|Default|GetTargetRotation2) _newtrack_0) false false))))

(event EventBeginPlay)

(event Collision|EventActorBeginOverlap
  (params (OtherActor :type Actor%20Object%20Reference)))

(event EventTick
  (params (DeltaSeconds :type Float%20%28single-precision%29)))

(fn ConstructionScript)