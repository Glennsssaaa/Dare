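; BP_CleanableHouse is a house object among the water spell objects, with a widget that shows only when flagged for the tutorial.
; BeginPlay runs the parent logic, sets widget visibility from ForTutorial and turns off its shadow.
; Each tick, after the parent's tick, the widget takes pitch and roll from a look-at toward the player camera while yaw stays fixed, so it only partly billboards.
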(event EventBeginPlay
  (bind _widget (Variables|Default|GetWidget))
  (|CallParentFunction)
  (Rendering|SetVisibility _widget (Variables|Default|GetForTutorial) false)
  (Rendering|SetCastShadow _widget false))

(event EventTick
  (params (DeltaSeconds :type Float%20%28single-precision%29))
  (bind _returnvalue (Game|GetPlayerCameraManager 0))
  (bind _widget (Variables|Default|GetWidget))
  (bind _returnvalue_2 (Transformation|GetWorldLocation _widget))
  (bind _returnvalue_3 (Camera|GetCameraLocation _returnvalue))
  (bind _returnvalue_4 (Math|Rotator|FindLookatRotation _returnvalue_2 _returnvalue_3))
  (|CallParentFunction DeltaSeconds)
  (Transformation|SetWorldRotation (Variables|Default|GetWidget) (Math|Rotator|MakeRotator (.roll _returnvalue_4) (.pitch _returnvalue_4) 1.8e+02) false false))

(fn ConstructionScript
  (|CallParentFunction))