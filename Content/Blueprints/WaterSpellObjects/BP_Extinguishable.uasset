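; BP_Extinguishable is a burning object in the water spell set that can be put out gradually.
; Each DrawOnObject event shrinks the FireVFX component's world scale by a small fixed step.
; Once the scale's vector length falls below a threshold, the next event destroys the fire and Cube components and activates PoofVFX, leaving the actor itself in place.
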(event Custom|DrawOnObject
  (bind _firevfx (Variables|Default|GetFireVFX))
  (bind _returnvalue (Transformation|GetWorldScale _firevfx))
  ;[1 1 1] Temp
  (if (< (Math|Vector|VectorLength _returnvalue) 2.0)
    (Components|DestroyComponent (Variables|Default|GetFireVFX))
    (Components|Activation|Activate (Variables|Default|GetPoofVFX) false)
    (Components|DestroyComponent (Variables|Default|GetCube))
    (else
      (Transformation|SetWorldScale3D _firevfx (- _returnvalue "0.100000,0.100000,0.100000")))))

(fn ConstructionScript)