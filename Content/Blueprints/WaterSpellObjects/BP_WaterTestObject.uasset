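; Dirty object that is cleaned by water spray and awards score when finished.
; BeginPlay creates a render target that the dirt material samples alongside clean and dirt textures.
; DrawOnObject paints spray marks into that target and adds CleanSpeed to CleanPercentage per call, without measuring coverage.
; At 100 percent it fills the target white and once triggers poof VFX, updates score and hides the widget if the object is a BP_CleanableHouse.
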(event Custom|DrawOnObject
  (params (Location%20To%20Draw :type Vector%202D%20Structure))
  (bind _rendertarget (Variables|Default|GetRenderTarget))
  (bind _watermarker_mi (Variables|Default|GetwaterMarker_MI))
  (if (>= (Variables|Default|GetCleanPercentage) 1e+02)
    ;[1 1 1] Finished Cleaning
    (Rendering|ClearRenderTarget2D _rendertarget "(R=1.000000,G=1.000000,B=1.000000,A=1.000000)")
    (Utilities|FlowControl|DoOnce false
      (:Completed
        (Components|Activation|Activate (Variables|Default|GetPoofVFX) false)
        (bind _returnvalue (Actor|GetActorOfClass "/Script/Dare.DareGameModeBase"))
        (Class|DareGameModeBase|UpdateScore _returnvalue (Variables|Default|GetPoints))
        (bind _asbp_cleanable_house (Utilities|Casting|CastToBP_CleanableHouse self))
        (Rendering|SetVisibility (Variables|/Game/Blueprints/WaterSpellObjects/BP_CleanableHouse.BP_CleanableHouse_C|GetWidget _asbp_cleanable_house) false false)))
    (else
      ;[1 1 1] Cleaning Render Target
      (Rendering|Material|SetVectorParameterValue _watermarker_mi "DrawLocation" (Math|Conversions|ToLinearColor(Vector) (Math|Conversions|ToVector(Vector2D) Location%20To%20Draw)) :!class /Script/Engine.MaterialInstanceDynamic)
      (Rendering|DrawMaterialtoRenderTarget _rendertarget _watermarker_mi)
      (Variables|Default|SetCleanPercentage (+ (Variables|Default|GetCleanPercentage) (Variables|Default|GetCleanSpeed))))))

(event EventBeginPlay
  ;[1 1 1] Initialise Materials & Render Target
  (bind _returnvalue (CanvasRenderTarget2D|CreateCanvasRenderTarget2D "/Script/Engine.CanvasRenderTarget2D" 1024 1024))
  (Variables|Default|SetRenderTarget _returnvalue)
  (bind _returnvalue_2 (Rendering|Material|CreateDynamicMaterialInstance "/Game/Materials/M_WaterSpray.M_WaterSpray" "None" "None" :!class /Script/Engine.KismetMaterialLibrary))
  (Variables|Default|SetwaterMarker_MI _returnvalue_2)
  (bind _returnvalue_3 (Rendering|Material|CreateDynamicMaterialInstance "/Game/Materials/M_DirtObject.M_DirtObject" "None" "None" :!class /Script/Engine.KismetMaterialLibrary))
  (Rendering|Material|SetTextureParameterValue _returnvalue_3 "RenderTargetVariable" (Variables|Default|GetRenderTarget))
  (Rendering|Material|SetTextureParameterValue _returnvalue_3 "CleanTexture" (Variables|Default|GetCleanTexture))
  (Rendering|Material|SetTextureParameterValue _returnvalue_3 "DirtTexture" (Variables|Default|GetDirtTexture))
  (Rendering|Material|SetMaterial (Variables|Default|GetCube) 0 _returnvalue_3)
  (Rendering|ClearRenderTarget2D "/Game/RT_DirtObject.RT_DirtObject"))

(fn ConstructionScript)