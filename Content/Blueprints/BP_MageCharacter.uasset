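; BP_MageCharacter is a mage character Blueprint whose graph drives a shared camera boom for two local players.
; On the first Tick it caches player characters 0 and 1 through a DoOnce.
; Every Tick it moves its SpringArm to their XY midpoint with a fixed X offset, keeping the arm's height.
; The clamped distance between both players sets the arm length, zooming out as they separate.
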(event EventBeginPlay)

(event Collision|EventActorBeginOverlap
  (params (OtherActor :type Actor%20Object%20Reference)))

(event EventTick
  (params (DeltaSeconds :type Float%20%28single-precision%29))
  (Utilities|FlowControl|Sequence
    (:then_0
      (Utilities|FlowControl|DoOnce false
        (:Completed
          (Variables|Default|SetTarget%20Actor (Game|GetPlayerCharacter 0))
          (Variables|Default|SetTarget%20Actor%202 (Game|GetPlayerCharacter 1)))))
    (:then_1
      (Transformation|SetWorldLocation (Variables|Default|GetSpringArm) (Math|Vector|MakeVector (- (.x (Math|Vector|Lerp(Vector) (Transformation|GetActorLocation (Variables|Default|GetTarget%20Actor)) (Transformation|GetActorLocation (Variables|Default|GetTarget%20Actor%202)) 0.5)) 5e+02) (.y (Math|Vector|Lerp(Vector) (Transformation|GetActorLocation (Variables|Default|GetTarget%20Actor)) (Transformation|GetActorLocation (Variables|Default|GetTarget%20Actor%202)) 0.5)) (.z (Transformation|GetWorldLocation (Variables|Default|GetSpringArm)))) false false)
      (Variables|/Script/Engine.SpringArmComponent|SetTargetArmLength (Variables|Default|GetSpringArm) (Math|Float|Clamp(Float) (Math|Vector|Distance(Vector) (Transformation|GetActorLocation (Variables|Default|GetTarget%20Actor%202)) (Transformation|GetActorLocation (Variables|Default|GetTarget%20Actor))) 2e+03 6e+03)))))

(fn ConstructionScript)