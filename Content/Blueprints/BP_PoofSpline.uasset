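; Scripted cutscene actor that sends a poof trail along a spline, wrecking scenery as it goes, then loads the playable first level.
; ActivateSpline shows the cutscene widget and plays a timeline that moves the sphere along the spline.
; Hardcoded distance thresholds swap materials and meshes to burnt or broken versions and fire Niagara effects.
; Late in the timeline, or on a gamepad skip, it starts the transition widget and opens the level.
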(event Custom|ActivateSpline
  (bind _spline (Variables|Default|GetSpline))
  (bind _returnvalue (UserInterface|CreateWidget "/Game/UI/WBP_Cutscene.WBP_Cutscene_C"))
  (UserInterface|Viewport|AddtoViewport _returnvalue 0)
  (Components|Activation|Activate (Variables|Default|GetP_PoofTrail) false)
  (Components|Timeline|SetPlayRate (Variables|Default|GetSplineTimeline) (/ 1.0 (Variables|Default|GetTimeToComplete)))
  (bind _newtrack_0 (Timeline|SplineTimeline Play)
    (:Update
      (Utilities|FlowControl|Sequence
        (:then_0
          (Transformation|SetWorldLocation (Variables|Default|GetSphere) (Spline|GetLocationatDistanceAlongSpline _spline (Math|Float|Lerp 0.0 (Spline|GetSplineLength _spline) _newtrack_0) "World") false false)
          (if (> (Math|Float|Lerp 0.0 (Spline|GetSplineLength _spline) _newtrack_0) 1e+03)
            (Rendering|Material|SetMaterial (Variables|/Script/Engine.StaticMeshActor|GetStaticMeshComponent (Utilities|Array|Get(acopy) (Variables|Default|GetMeshes))) 0 "/Game/Materials/MI_TreeTrunk_Burnt.MI_TreeTrunk_Burnt")
            (Components|Activation|Activate (Variables|/Script/Niagara.NiagaraActor|GetNiagaraComponent (Utilities|Array|Get(acopy) (Variables|Default|GetVFX))) false)
            (if (> (Math|Float|Lerp 0.0 (Spline|GetSplineLength _spline) _newtrack_0) 2.5e+03)
              (Components|StaticMesh|SetStaticMesh (Variables|/Script/Engine.StaticMeshActor|GetStaticMeshComponent (Utilities|Array|Get(acopy) (Variables|Default|GetMeshes) 1)) "/Game/Assets/Environment/BrokenHouseA.BrokenHouseA")
              (Components|Activation|Activate (Variables|/Script/Niagara.NiagaraActor|GetNiagaraComponent (Utilities|Array|Get(acopy) (Variables|Default|GetVFX) 1)) false)
              (if (> (Math|Float|Lerp 0.0 (Spline|GetSplineLength _spline) _newtrack_0) 3e+03)
                (Components|Activation|Activate (Variables|/Script/Niagara.NiagaraActor|GetNiagaraComponent (Utilities|Array|Get(acopy) (Variables|Default|GetVFX) 2)) false)
                (if (> (Math|Float|Lerp 0.0 (Spline|GetSplineLength _spline) _newtrack_0) 8e+03)
                  (Components|StaticMesh|SetStaticMesh (Variables|/Script/Engine.StaticMeshActor|GetStaticMeshComponent (Utilities|Array|Get(acopy) (Variables|Default|GetMeshes) 2)) "/Game/Assets/Environment/BrokenHouseA.BrokenHouseA")
                  (Components|Activation|Activate (Variables|/Script/Niagara.NiagaraActor|GetNiagaraComponent (Utilities|Array|Get(acopy) (Variables|Default|GetVFX) 3)) false)
                  (if (> (Math|Float|Lerp 0.0 (Spline|GetSplineLength _spline) _newtrack_0) 8e+03)
                    (Components|Activation|Activate (Variables|/Script/Niagara.NiagaraActor|GetNiagaraComponent (Utilities|Array|Get(acopy) (Variables|Default|GetVFX) 4)) false)
                    (if (> (Math|Float|Lerp 0.0 (Spline|GetSplineLength _spline) _newtrack_0) 8e+03)
                      (Components|Activation|Activate (Variables|/Script/Niagara.NiagaraActor|GetNiagaraComponent (Utilities|Array|Get(acopy) (Variables|Default|GetVFX) 5)) false)
                      (if (> (Math|Float|Lerp 0.0 (Spline|GetSplineLength _spline) _newtrack_0) 8e+03)
                        (Components|Activation|Activate (Variables|/Script/Niagara.NiagaraActor|GetNiagaraComponent (Utilities|Array|Get(acopy) (Variables|Default|GetVFX) 6)) false)
                        (if (> (Math|Float|Lerp 0.0 (Spline|GetSplineLength _spline) _newtrack_0) 8e+03)
                          (Components|Activation|Activate (Variables|/Script/Niagara.NiagaraActor|GetNiagaraComponent (Utilities|Array|Get(acopy) (Variables|Default|GetVFX) 7)) false))))))))))
        (:then_1
          (if (not (< _newtrack_0 0.75))
            (Variables|/Game/UI/WBP_Transition.WBP_Transition_C|SetStartTransition (Variables|Default|GetTransitionWidget) true)
            (Widget|RemovefromParent _returnvalue)
            (Utilities|FlowControl|Delay 2.0)
            (Actor|DestroyActor)
            (Game|OpenLevel(byObjectReference) "/Game/Levels/Level1Playable.Level1Playable")))))))

(event EventBeginPlay
  (bind _returnvalue (UserInterface|CreateWidget "/Game/UI/WBP_Transition.WBP_Transition_C"))
  (bind _output_get (Variables|Default|SetTransitionWidget _returnvalue))
  (UserInterface|Viewport|AddtoViewport _returnvalue 0))

(event Collision|EventActorBeginOverlap
  (params (OtherActor :type Actor%20Object%20Reference)))

(event EventTick
  (params (DeltaSeconds :type Float%20%28single-precision%29))
  (if (Game|Player|WasInputKeyJustPressed (Game|GetPlayerController 0) "Gamepad_FaceButton_Right")
    (Variables|/Game/UI/WBP_Transition.WBP_Transition_C|SetStartTransition (Variables|Default|GetTransitionWidget) true)
    (Widget|RemovefromParent (stale Custom|ActivateSpline _returnvalue))
    (Utilities|FlowControl|Delay 2.0)
    (Actor|DestroyActor)
    (Game|OpenLevel(byObjectReference) "/Game/Levels/Level1Playable.Level1Playable")))

(fn ConstructionScript)