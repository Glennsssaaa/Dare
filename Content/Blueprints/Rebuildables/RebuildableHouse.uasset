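; Rebuildable house that displays a rebuild progress bar through its widget component.
; Overlap events on RebuildCollision show the widget on begin and hide it on end, with no filter on the overlapping actor.
; BeginPlay caches the widget as a RebuildProgressBar, and Tick copies RebuildProgress into its percentage every frame.
; This graph only reads RebuildProgress and never changes it.
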(event OnComponentBeginOverlap(RebuildCollision)
  (params (OverlappedComponent :type Primitive%20Component%20Object%20Reference) (OtherActor :type Actor%20Object%20Reference) (OtherComp :type Primitive%20Component%20Object%20Reference) (OtherBodyIndex :type Integer) (bFromSweep :type Boolean) (SweepResult :type Hit%20Result%20Structure%20%28by%20ref%29))
  (Rendering|SetVisibility (Variables|Default|GetWidget) true false))

(event OnComponentEndOverlap(RebuildCollision)
  (params (OverlappedComponent :type Primitive%20Component%20Object%20Reference) (OtherActor :type Actor%20Object%20Reference) (OtherComp :type Primitive%20Component%20Object%20Reference) (OtherBodyIndex :type Integer))
  (Rendering|SetVisibility (Variables|Default|GetWidget) false false))

(event EventBeginPlay
  (bind _asrebuild_progress_bar (Utilities|Casting|CastToRebuildProgressBar (UserInterface|GetUserWidgetObject (Variables|Default|GetWidget))))
  (Variables|Default|SetProgressRef _asrebuild_progress_bar))

(event EventTick
  (params (DeltaSeconds :type Float%20%28single-precision%29))
  (Variables|/Game/Blueprints/UIWidgets/RebuildProgressBar.RebuildProgressBar_C|SetRebuildPercentage (Variables|Default|GetProgressRef) (Variables|Default|GetRebuildProgress)))

(fn ConstructionScript)