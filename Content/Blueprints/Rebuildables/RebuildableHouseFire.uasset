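; Rebuildable house that starts as a fire hazard the player puts out by drawing on it before it can be rebuilt.
; Each draw shrinks the fire; once small enough it is removed with a poof, Points are halved and awarded, and IsOnFire clears.
; Overlap then toggles the progress bar, while Tick feeds it RebuildProgress, triggers poof effects and turns the tutorial tip toward the camera with fixed yaw.
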(event OnComponentBeginOverlap(RebuildCollision)
  (params (OverlappedComponent :type Primitive%20Component%20Object%20Reference) (OtherActor :type Actor%20Object%20Reference) (OtherComp :type Primitive%20Component%20Object%20Reference) (OtherBodyIndex :type Integer) (bFromSweep :type Boolean) (SweepResult :type Hit%20Result%20Structure%20%28by%20ref%29))
  (if (not (Variables|Default|GetbIsOnFire))
    (Rendering|SetVisibility (Variables|Default|GetProgressBar) true false)))

(event OnComponentEndOverlap(RebuildCollision)
  (params (OverlappedComponent :type Primitive%20Component%20Object%20Reference) (OtherActor :type Actor%20Object%20Reference) (OtherComp :type Primitive%20Component%20Object%20Reference) (OtherBodyIndex :type Integer))
  (if (not (Variables|Default|GetbIsOnFire))
    (Rendering|SetVisibility (Variables|Default|GetProgressBar) false false)))

(event Custom|DrawOnObject
  (bind _firevfx1 (Variables|Default|GetFireVFX1))
  (bind _returnvalue (Transformation|GetWorldScale _firevfx1))
  ;[1 1 1] Temp
  (if (Variables|Default|GetbIsOnFire)
    (if (< (Math|Vector|VectorLength _returnvalue) 2.0)
      (Components|DestroyComponent (Variables|Default|GetFireVFX1))
      (Components|Activation|Activate (Variables|Default|GetPoofVFX1) false)
      (Components|DestroyComponent (Variables|Default|GetCube))
      (bind _returnvalue_2 (Actor|GetActorOfClass "/Script/Dare.DareGameModeBase"))
      (Variables|Default|SetPoints (/ (Variables|Default|GetPoints) 2.0))
      (Class|DareGameModeBase|UpdateScore _returnvalue_2 (Variables|Default|GetPoints))
      (Variables|Default|SetbIsOnFire false)
      (else
        (Transformation|SetWorldScale3D _firevfx1 (- _returnvalue "0.200000,0.200000,0.200000"))))))

(event EventBeginPlay
  (bind _asrebuild_progress_bar (Utilities|Casting|CastToRebuildProgressBar (UserInterface|GetUserWidgetObject (Variables|Default|GetProgressBar))))
  (Variables|Default|SetProgressRef _asrebuild_progress_bar)
  (Rendering|SetVisibility (Variables|Default|GetTutorialTip) (Variables|Default|GetbForTutorial) false))

(event EventTick
  (params (DeltaSeconds :type Float%20%28single-precision%29))
  (bind _returnvalue (Game|GetPlayerCameraManager 0))
  (bind _rebuildprogress (Variables|Default|GetRebuildProgress))
  (bind _tutorialtip (Variables|Default|GetTutorialTip))
  (bind _returnvalue_2 (Transformation|GetWorldLocation _tutorialtip))
  (bind _returnvalue_3 (Camera|GetCameraLocation _returnvalue))
  (bind _returnvalue_4 (Math|Rotator|FindLookatRotation _returnvalue_2 _returnvalue_3))
  (Utilities|FlowControl|Sequence
    (:then_0
      (Transformation|SetWorldRotation (Variables|Default|GetTutorialTip) (Math|Rotator|MakeRotator (.roll _returnvalue_4) (.pitch _returnvalue_4) 1.8e+02) false false))
    (:then_1
      (if (not (Variables|Default|GetbIsOnFire))
        (Utilities|FlowControl|Sequence
          (:then_0
            (bind _output_get (Variables|/Game/Blueprints/UIWidgets/RebuildProgressBar.RebuildProgressBar_C|SetRebuildPercentage (Variables|Default|GetProgressRef) _rebuildprogress))
            (if (Variables|Default|GetbIsRebuilding)
              (Components|Activation|Activate (Variables|Default|GetPoofVFX) true)
              (else
                (Utilities|FlowControl|DoOnce false)))))))
    (:then_2
      (if (== _rebuildprogress 0.0)
        (Utilities|FlowControl|DoOnce false :!label _label
          (:Completed
            (Components|Activation|Activate (Variables|Default|GetPoofVFX) true)))
        (else
          (goto _label Reset))))))

(fn ConstructionScript)