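; BP_Camera is a shared camera, marked temporary, that frames the Mage and Tank player characters.
; On its first Tick it caches players 0 and 1 as the two characters.
; Every Tick it moves the spring arm to their midpoint with a fixed X offset, keeping the height recorded at BeginPlay.
; It zooms by setting arm length to the distance between them, clamped to a range.
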(event EventBeginPlay
  (Variables|Default|SetSpringArmZ (.z (Transformation|GetWorldLocation (Variables|Default|GetSpringArm)))))

(event EventTick
  (params (DeltaSeconds :type Float%20%28single-precision%29))
  ;[1 1 1] Camera Movement (Temp)
  (Utilities|FlowControl|Sequence
    (:then_0
      (Utilities|FlowControl|DoOnce false
        (:Completed
          (Variables|Default|SetMageCharacter (Game|GetPlayerCharacter 0))
          (Variables|Default|SetTankCharacter (Game|GetPlayerCharacter 1)))))
    (:then_1
      (Transformation|SetWorldLocation (Variables|Default|GetSpringArm) (Math|Vector|MakeVector (- (.x (Math|Vector|Lerp(Vector) (Transformation|GetActorLocation (Variables|Default|GetMageCharacter)) (Transformation|GetActorLocation (Variables|Default|GetTankCharacter)) 0.5)) 5e+02) (.y (Math|Vector|Lerp(Vector) (Transformation|GetActorLocation (Variables|Default|GetMageCharacter)) (Transformation|GetActorLocation (Variables|Default|GetTankCharacter)) 0.5)) (Variables|Default|GetSpringArmZ)) false false)
      (Variables|/Script/Engine.SpringArmComponent|SetTargetArmLength (Variables|Default|GetSpringArm) (Math|Float|Clamp(Float) (Math|Vector|Distance(Vector) (Transformation|GetActorLocation (Variables|Default|GetMageCharacter)) (Transformation|GetActorLocation (Variables|Default|GetTankCharacter))) 2.5e+03 7.5e+03)))))

(fn ConstructionScript)