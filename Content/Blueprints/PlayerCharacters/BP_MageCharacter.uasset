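; Mage player character that casts water at objects to paint, extinguish or grow them.
; BeginPlay moves it to the "MageSpawn" player start and attaches a spawned broom to a mesh socket.
; DrawFunc aims the water VFX from the right hand to the hit position and forwards hits by casting to each target type.
; Tick caches both player characters once and toggles the VFX, while left click plays a cast montage.
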(event EventBeginPlay
  ;[1 1 1] Spawn Location Setter
  (Transformation|SetActorTransform (Math|Transform|MakeTransform (Transformation|GetActorLocation (Class|GameModeBase|FindPlayerStart (Game|GetGameMode) (Game|GetPlayerController 0) "MageSpawn")) "0, 0, 0" "1.000000,1.000000,1.000000"))
  (bind _returnvalue (Game|SpawnActorfromClass "/Game/Assets/Characters/Witch/Broom/BP_Broom.BP_Broom_C" (Transformation|GetSocketTransform (Variables|Default|GetPlayerMesh) "BroomSocket" "RTS_World") "Undefined" 0 0))
  (Transformation|AttachComponentToComponent _returnvalue (Variables|Default|GetPlayerMesh) "BroomSocket" "SnapToTarget" "SnapToTarget" "SnapToTarget" true))

(event EventDrawFunc
  (params (hitActor :type Actor%20Object%20Reference) (hitUV :type Vector%202D%20Structure))
  (bind _watervfx (Variables|Default|GetWaterVFX))
  (bind _playermesh (Variables|Default|GetPlayerMesh))
  ;[1 1 1] Water Drawing Event
  (Niagara|SetNiagaraVariable(Vector3) _watervfx "StartLocation" (Transformation|GetSocketLocation _playermesh (Class|SkinnedMeshComponent|GetSocketBoneName _playermesh "jnt_R_fingers_01")))
  (Niagara|SetNiagaraVariable(Vector3) _watervfx "TargetVector" (Variables|Default|GetWaterHitPosition))
  (bind _asbp_water_test_object (Utilities|Casting|CastToBP_WaterTestObject hitActor)
    (:then
      (Default|DrawonObject _asbp_water_test_object hitUV))
    (:CastFailed
      (bind _asbp_extinguishable (Utilities|Casting|CastToBP_Extinguishable hitActor)
        (:then
          (Default|DrawonObject _asbp_extinguishable))
        (:CastFailed
          (bind _asbp_growing_object (Utilities|Casting|CastToBP_GrowingObject hitActor))
          (Default|DrawonObject _asbp_growing_object))))))

(event EventTick
  (params (DeltaSeconds :type Float%20%28single-precision%29))
  (Utilities|FlowControl|Sequence
    (:then_0
      ;[1 1 1] Controller Setup
      (Utilities|FlowControl|DoOnce false
        (:Completed
          (Variables|Default|SetTarget%20Actor (Game|GetPlayerCharacter 0))
          (Variables|Default|SetTarget%20Actor%202 (Game|GetPlayerCharacter 1)))))
    (:then_1
      (if (Variables|Default|GetbEnableWaterVFX)
        (Class|NiagaraComponent|SetVariableBool (Variables|Default|GetWaterVFX) "bIsActive" true)
        (else
          (Class|NiagaraComponent|SetVariableBool (Variables|Default|GetWaterVFX) "bIsActive" false))))))

(event Input|MouseEvents|LeftMouseButton
  (params (Key :type Key%20Structure :default "None"))
  (:Pressed
    (Development|PrintString "Hello")
    (Animation|Montage|PlayMontage (Variables|Default|GetPlayerMesh) "/Game/Assets/Characters/Witch/WalkCastLoop.WalkCastLoop")))

(fn ConstructionScript)