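; Player controller that provides a key remap menu doubling as a pause screen on the P key.
; After short startup delays it caches the Enhanced Input player-mappable mappings and the character's default mapping context, then creates the remap widget from the default mappings.
; A FlipFlop on P alternates between showing the menu with the game paused and removing it to unpause; the mouse cursor is enabled but never hidden again.
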(event Custom|Create%20Key%20Select
  (Utilities|FlowControl|Delay 1.0)
  (bind _returnvalue (UserInterface|CreateWidget "/Game/Blueprints/UIWidgets/Remapping/RemapList.RemapList_C"))
  (bind _output_get (Variables|Default|SetRemapMenuRef _returnvalue))
  (Default|RefreshMappings _output_get (Variables|Default|GetDefaultMappings)))

(event EventBeginPlay
  (Utilities|FlowControl|Delay 1.0)
  (Variables|Default|SetMappings (CallFunction|GetAllMappings))
  (Variables|Default|SetDefaultMappings (Variables|/Script/EnhancedInput.InputMappingContext|GetMappings (Variables|/Script/Dare.APlayerCharacter|GetDefaultMappingContext (.AsAPlayer%20Character (Utilities|Casting|CastToAPlayerCharacter (Game|GetPlayerCharacter 0))))))
  (CallFunction|CreateKeySelect))

(event Input|KeyboardEvents|P
  (params (Key :type Key%20Structure :default "None"))
  (bind _remapmenuref (Variables|Default|GetRemapMenuRef))
  ;[1 1 1] Pause
  (:Pressed
    (Utilities|FlowControl|FlipFlop
      (:A
        (UserInterface|Viewport|AddtoViewport _remapmenuref 0)
        (Game|SetGamePaused true)
        (Variables|Default|SetbShowMouseCursor true))
      (:B
        (Widget|RemovefromParent _remapmenuref)
        (Game|SetGamePaused false)))))

(fn ConstructionScript)

(fn GetAllMappings
  (return (Class|EnhancedInputSubsystemInterface|GetAllPlayerMappableActionKeyMappings (PlayerController|LocalPlayerSubsystems|GetEnhancedInputLocalPlayerSubsystem))))