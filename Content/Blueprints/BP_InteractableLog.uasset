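; An interactable log that can either be toppled like a tree or broken apart.
; It outlines its cylinders through custom depth on overlap while MuscleOverlap is set, and clears the outline and flag on end overlap.
; Interact with Pushtree set enables a Tick-driven lerp toward a hardcoded fallen location and rotation.
; Otherwise Interact launches both boxes with physics impulses and destroys the actor after a short delay.
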(event Custom|Interact
  (bind _box1 (Variables|Components|GetBox1))
  (if (Variables|Default|GetPushtree)
    (Variables|Default|SetEnableFalling true)
    (else
      (Physics|SetSimulatePhysics (Variables|Components|GetBox) true)
      (Physics|AddImpulse (Variables|Components|GetBox) "-350.000000,600.000000,1.000000" "None" true)
      (Physics|SetSimulatePhysics _box1 true)
      (Physics|AddImpulse _box1 "300.000000,600.000000,1.000000" "None" true)
      (Utilities|FlowControl|Delay 2.0)
      (Actor|DestroyActor))))

(event EventBeginPlay)

(event Collision|EventActorBeginOverlap
  (params (OtherActor :type Actor%20Object%20Reference))
  (if (Variables|Default|GetMuscleOverlap)
    (Rendering|SetRenderCustomDepth (Variables|Components|GetCylinder) true)
    (Rendering|SetRenderCustomDepth (Variables|Components|GetCylinder1) true)))

(event Collision|EventActorEndOverlap
  (params (OtherActor :type Actor%20Object%20Reference))
  (Rendering|SetRenderCustomDepth (Variables|Components|GetBox) false)
  (Rendering|SetRenderCustomDepth (Variables|Components|GetBox1) false)
  (Variables|Default|SetMuscleOverlap false))

(event EventTick
  (params (DeltaSeconds :type Float%20%28single-precision%29))
  (if (Variables|Default|GetEnableFalling)
    (Transformation|SetActorLocationAndRotation (Math|Vector|Lerp(Vector) (Transformation|GetActorLocation) "451.000000,6415.000000,-91.000000" 0.01) (Math|Rotator|Lerp(Rotator) (Transformation|GetActorRotation) "0.000000,90.000000,-90.000000" 0.01 true))))

(fn ConstructionScript)