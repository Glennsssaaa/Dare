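; BP_GrowingObject2 is a growable earth-spell object with an optional tutorial widget, shown at start only when ForTutorial is set.
; Tick watches HasGrown and, the first time it is true, fires the poof VFX and hides the widget.
; Every tick also tilts the widget toward the player camera using look-at pitch and roll, with yaw locked at 180 degrees.
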(event EventBeginPlay
  (bind _tutorialwidget (Variables|Default|GetTutorialWidget))
  (Rendering|SetVisibility _tutorialwidget (Variables|Default|GetForTutorial) false)
  (Rendering|SetCastShadow _tutorialwidget false))

(event EventTick
  (params (DeltaSeconds :type Float%20%28single-precision%29))
  (bind _returnvalue (Game|GetPlayerCameraManager 0))
  (bind _tutorialwidget (Variables|Default|GetTutorialWidget))
  (bind _returnvalue_2 (Transformation|GetWorldLocation _tutorialwidget))
  (bind _returnvalue_3 (Camera|GetCameraLocation _returnvalue))
  (bind _returnvalue_4 (Math|Rotator|FindLookatRotation _returnvalue_2 _returnvalue_3))
  (Utilities|FlowControl|Sequence
    (:then_0
      (if (Variables|Default|GethasGrown)
        (Utilities|FlowControl|DoOnce false
          (:Completed
            (Components|Activation|Activate (Variables|Default|GetPoofVFX) false)
            (Rendering|SetVisibility (Variables|Default|GetTutorialWidget) false false)))))
    (:then_1
      (Transformation|SetWorldRotation (Variables|Default|GetTutorialWidget) (Math|Rotator|MakeRotator (.roll _returnvalue_4) (.pitch _returnvalue_4) 1.8e+02) false false))))

(fn ConstructionScript)