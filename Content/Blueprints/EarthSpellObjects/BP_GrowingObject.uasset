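; Earth spell object that grows in fixed steps each time its DrawOnObject event is called, marked as temporary.
; Each call enlarges the whole actor evenly until the vector length of the Cube's world scale exceeds a threshold.
; The first call after that activates PoofVFX instead of growing, and a flag keeps the effect from being triggered again.
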(event Custom|DrawOnObject
  ;[1 1 1] Temp
  (if (> (Math|Vector|VectorLength (Transformation|GetWorldScale (Variables|Default|GetCube))) 1.0)
    (if (not (Variables|Default|GetVFXActivated))
      (Components|Activation|Activate (Variables|Default|GetPoofVFX) false)
      (Variables|Default|SetVFXActivated true))
    (else
      (Transformation|SetActorScale3D (+ (Transformation|GetActorScale3D) "0.250000,0.250000,0.250000")))))

(fn ConstructionScript)