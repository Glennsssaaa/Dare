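; BP_GrowingFlower is an earth spell object: three flower meshes that grow and award score when finished.
; BeginPlay creates one dynamic flower-card material shared by all three meshes.
; While CurrentlyGrowing is set, Tick increments Growth at a frame-rate-dependent rate, driving a material parameter and each mesh's morph target.
; Once Growth passes full, it fires a poof VFX and adds Points through DareGameModeBase, guarded to run once.
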(event EventBeginPlay
  (bind _returnvalue (Rendering|Material|CreateDynamicMaterialInstance (Variables|Default|GetFlower) 0 "/Game/Materials/MI_FlowerCard.MI_FlowerCard" "None" :!class /Script/Engine.PrimitiveComponent))
  (Rendering|Material|SetMaterial (Variables|Default|GetFlower1) 0 _returnvalue)
  (Rendering|Material|SetMaterial (Variables|Default|GetFlower2) 0 _returnvalue))

(event EventTick
  (params (DeltaSeconds :type Float%20%28single-precision%29))
  ;[1 1 1] Temp
  (if (Variables|Default|GetCurrentlyGrowing)
    (if (> (Variables|Default|GetGrowth) 1.0)
      (if (not (Variables|Default|GetVFXActivated))
        (Components|Activation|Activate (Variables|Default|GetPoofVFX) false)
        (Variables|Default|SetVFXActivated true)
        (bind _returnvalue (Actor|GetActorOfClass "/Script/Dare.DareGameModeBase"))
        (Class|DareGameModeBase|UpdateScore _returnvalue (Variables|Default|GetPoints)))
      (else
        (Rendering|Material|SetScalarParameterValue (stale EventBeginPlay _returnvalue) "Growth" (Variables|Default|GetGrowth) :!class /Script/Engine.MaterialInstanceDynamic)
        (bind _output_get (Variables|Default|SetGrowth (+ (Variables|Default|GetGrowth) 0.01)))
        (Components|SkeletalMesh|SetMorphTarget (Variables|Default|GetFlower) "YellowFlower1_FinalState" _output_get true)
        (Components|SkeletalMesh|SetMorphTarget (Variables|Default|GetFlower1) "YellowFlower1_FinalState" _output_get true)
        (Components|SkeletalMesh|SetMorphTarget (Variables|Default|GetFlower2) "YellowFlower1_FinalState" _output_get true)))))

(fn ConstructionScript)