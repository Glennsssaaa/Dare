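; Earth spell bridge object that, once interacted with, slides four lilypads into place as a bridge.
; Lilypads start without collision; Tick clears their custom depth and interpolates their local Y toward zero.
; When a lilypad nears its target, collision is enabled on those still in the array and it is removed.
; Once the array empties, Tick stops, the mage is unfrozen, ObjectMesh is hidden and the game mode's MageTutorialObject is called.
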(event EventBeginPlay
  (bind _lilypads (Variables|Default|GetLilypads))
  (Utilities|Array|Add _lilypads (Variables|Default|GetLilypad4))
  (Utilities|Array|Add _lilypads (Variables|Default|GetLilypad3))
  (Utilities|Array|Add _lilypads (Variables|Default|GetLilypad2))
  (Utilities|Array|Add _lilypads (Variables|Default|GetLilypad1))
  (for _array_element (Variables|Default|GetLilypads)
    (Collision|SetCollisionEnabled _array_element "NoCollision")))

(event EventTick
  (params (DeltaSeconds :type Float%20%28single-precision%29))
  (bind _lilypads (Variables|Default|GetLilypads))
  (if (Variables|Default|GetbInteracted)
    (if (> (Utilities|Array|Length (Variables|Default|GetLilypads)) 0)
      (for _array_element (Variables|Default|GetLilypads)
        (Rendering|SetRenderCustomDepth _array_element false)
        (Transformation|SetRelativeLocation _array_element (Math|Interpolation|VInterpTo (Variables|/Script/Engine.SceneComponent|GetRelativeLocation _array_element) (Math|Vector|MakeVector (.x (Variables|/Script/Engine.SceneComponent|GetRelativeLocation _array_element)) 0.0 (.z (Variables|/Script/Engine.SceneComponent|GetRelativeLocation _array_element))) DeltaSeconds 2.0) false false)
        (if (Math|Float|NearlyEqual(Float) (.y (Variables|/Script/Engine.SceneComponent|GetRelativeLocation _array_element)) 0.0 3.0)
          (for _array_element_2 _lilypads
            (Collision|SetCollisionEnabled _array_element_2 "QueryAndPhysics"))
          (Utilities|Array|RemoveItem _lilypads _array_element)))
      (else
        (Actor|Tick|SetActorTickEnabled false)
        (Variables|Default|SetbFreezePlayer false)
        (bind _outactors (Actor|GetAllActorsOfClass "/Game/Blueprints/PlayerCharacters/BP_MageCharacter.BP_MageCharacter_C"))
        (Variables|/Script/Dare.PlayerCharacter|SetbPlayerFrozen (Utilities|Array|Get(acopy) _outactors) false)
        (Rendering|SetVisibility (Variables|Default|GetObjectMesh) false false)
        (bind _returnvalue (Actor|GetActorOfClass "/Script/Dare.DareGameModeBase"))
        (Class|DareGameModeBase|MageTutorialObject _returnvalue)))))

(fn ConstructionScript)