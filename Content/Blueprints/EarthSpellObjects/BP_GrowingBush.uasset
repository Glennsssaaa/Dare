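; BP_GrowingBush is an earth spell object: a bush the mage grows to earn score.
; Each tick, while colliding with the mage's earth toggle on, it increments Growth and plays leaf VFX, which otherwise switch off.
; Once Growth passes its threshold, it fires a one-time poof, hides the tutorial widget, adds Points through DareGameModeBase and swaps to the bush mesh.
; The mage is looked up every tick, and a debug print remains.
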(event EventTick
  (params (DeltaSeconds :type Float%20%28single-precision%29))
  (bind _returnvalue (Actor|GetActorOfClass "/Game/Blueprints/PlayerCharacters/BP_MageCharacter.BP_MageCharacter_C"))
  ;[1 1 1] Temp
  (if (and (Variables|Default|GetIsColliding) (Variables|/Script/Dare.MageCharacter|GetbToggleEarth _returnvalue))
    (Utilities|FlowControl|Sequence
      (:then_1
        (Development|PrintString "Hello")
        (if (> (Variables|Default|GetGrowth) 1.0)
          (if (not (Variables|Default|GetVFXActivated))
            (Components|Activation|Activate (Variables|Default|GetPoofVFX) false)
            (Variables|Default|SetVFXActivated true)
            (Rendering|SetVisibility (Variables|Default|GetTutorialWidget) false false)
            (Components|Activation|SetActive (Variables|Default|GetLeafVFX) false false)
            (bind _returnvalue_2 (Actor|GetActorOfClass "/Script/Dare.DareGameModeBase"))
            (Class|DareGameModeBase|UpdateScore _returnvalue_2 (Variables|Default|GetPoints))
            (Components|StaticMesh|SetStaticMesh (Variables|Default|GetObjectMesh) "/Game/Assets/Environment/SM_Bush.SM_Bush"))
          (else
            (Variables|Default|SetGrowth (+ (Variables|Default|GetGrowth) 0.01))
            (Components|Activation|SetActive (Variables|Default|GetLeafVFX) true false)))))
    (else
      (Components|Activation|SetActive (Variables|Default|GetLeafVFX) false false))))

(fn ConstructionScript)