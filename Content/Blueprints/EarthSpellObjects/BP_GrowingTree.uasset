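; BP_GrowingTree is an earth-spell object that grows into a pine tree while colliding and the mage's ToggleEarth is active.
; Tick swaps in the pine mesh at small scale once, then raises its scale each frame with leaf VFX playing.
; Once Growth passes full size, it stops the VFX and one time either notifies the game mode of a tutorial object or adds Points to the score.
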(event EventTick
  (params (DeltaSeconds :type Float%20%28single-precision%29))
  (bind _objectmesh (Variables|Default|GetObjectMesh))
  (bind _returnvalue (Actor|GetActorOfClass "/Game/Blueprints/PlayerCharacters/BP_MageCharacter.BP_MageCharacter_C"))
  ;[1 1 1] Temp
  (if (and (Variables|Default|GetIsColliding) (Variables|/Script/Dare.MageCharacter|GetbToggleEarth _returnvalue))
    (Utilities|FlowControl|Sequence
      (:then_0
        (Utilities|FlowControl|DoOnce false
          (:Completed
            (Components|StaticMesh|SetStaticMesh (Variables|Default|GetObjectMesh) "/Game/Assets/Environment/SM_PineTree.SM_PineTree")
            (Transformation|SetWorldScale3D (Variables|Default|GetObjectMesh) "0.100000,0.100000,0.100000")
            (Transformation|SetWorldScale3D (Variables|Default|GetCollisionMesh) "1.000000,1.000000,1.000000")
            (Rendering|SetVisibility (Variables|Default|GetTutorialWidget) false false))))
      (:then_1
        (if (> (Variables|Default|GetGrowth) 1.0)
          (if (not (Variables|Default|GetVFXActivated))
            (Variables|Default|SetVFXActivated true)
            (Rendering|SetVisibility (Variables|Default|GetTutorialWidget) false false)
            (Components|Activation|SetActive (Variables|Default|GetLeafVFX) false false)
            (bind _returnvalue_2 (Actor|GetActorOfClass "/Script/Dare.DareGameModeBase"))
            (if (Variables|Default|GetmageTutorialObject)
              (Class|DareGameModeBase|MageTutorialObject _returnvalue_2)
              (Rendering|SetVisibility (Variables|Default|GetTutorialWidget) false false)
              (else
                (Class|DareGameModeBase|UpdateScore _returnvalue_2 (Variables|Default|GetPoints)))))
          (else
            (Variables|Default|SetGrowth (.x (Transformation|GetWorldScale _objectmesh)))
            (Transformation|SetWorldScale3D _objectmesh (+ (Transformation|GetWorldScale _objectmesh) "0.005000,0.005000,0.005000"))
            (Components|Activation|SetActive (Variables|Default|GetLeafVFX) true false)
            (Transformation|SetWorldScale3D (Variables|Default|GetCollisionMesh) "1.000000,1.000000,1.000000")))))
    (else
      (Components|Activation|SetActive (Variables|Default|GetLeafVFX) false false))))

(fn ConstructionScript)