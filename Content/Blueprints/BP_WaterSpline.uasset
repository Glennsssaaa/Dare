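; BP_WaterSpline is an actor that sends a sphere along a spline path and then loads the Level1Playable level.
; ActivateSpline starts the PPoofTrail effect and plays a timeline with its rate set from TimeToComplete.
; Each update lerps the timeline value over the spline length to position the sphere in world space.
; When the timeline finishes, the actor destroys itself and opens the level.
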(event Custom|ActivateSpline
  (bind _spline (Variables|Default|GetSpline))
  (Components|Activation|Activate (Variables|Default|GetP_PoofTrail) false)
  (Components|Timeline|SetPlayRate (Variables|Default|GetSplineTimeline) (/ 1.0 (Variables|Default|GetTimeToComplete)))
  (bind _newtrack_0 (Timeline|SplineTimeline Play)
    (:Update
      (Transformation|SetWorldLocation (Variables|Default|GetSphere) (Spline|GetLocationatDistanceAlongSpline _spline (Math|Float|Lerp 0.0 (Spline|GetSplineLength _spline) _newtrack_0) "World") false false))
    (:Finished
      (Actor|DestroyActor)
      (Game|OpenLevel(byObjectReference) "/Game/Levels/Level1Playable.Level1Playable"))))

(event EventBeginPlay)

(event Collision|EventActorBeginOverlap
  (params (OtherActor :type Actor%20Object%20Reference)))

(fn ConstructionScript)